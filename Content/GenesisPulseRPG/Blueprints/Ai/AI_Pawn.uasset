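; AI controller that keeps its pawn wandering around the player's location in an endless loop.
; Each cycle picks a random reachable point near player 0, moves there with AIMoveTo, then restarts on success or retries after a short delay on failure.
; Alongside each new move, it randomly sends the pawn either a run toggle or jump and sprint toggle messages.
; GetLockedEnemy and OnAlertAI are empty stubs.
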(event `self.ReceiveBeginPlay`
  (bind _returnvalue (`KismetMathLibrary.RandomBool`))
  (bind _ch (`self.CH`))
  (set `self.CH` (`self.K2_GetPawn`))
  (`self.GoToLocation` (`NavigationSystemV1.K2_GetRandomReachablePointInRadius` (`self.K2_GetActorLocation` (`GameplayStatics.GetPlayerCharacter` 0)) 2000.0 null null) :!label _label)
  (if _returnvalue
    (message `/Game/GenesisPulseRPG/Blueprints/Interfrace/BPI_Chatracter.ToggleRun` _ch _returnvalue)
    (else
      (`|ExecutionSequence`
        (:`then_0`
          (message `/Game/GenesisPulseRPG/Blueprints/Interfrace/BPI_Chatracter.ToggleJump` _ch _returnvalue))
        (:`then_1`
          (message `/Game/GenesisPulseRPG/Blueprints/Interfrace/BPI_Chatracter.ToggleSprint` _ch _returnvalue))))))

(event `self.GoToLocation`
  (params (`target location` :type "Vector Structure"))
  (`|AIMoveTo` null (`NavigationSystemV1.K2_GetRandomReachablePointInRadius` `target location` 100.0 null null) null 200.0 :!label _label_2
    (:`OnSuccess`
      (goto _label))
    (:`OnFail`
      (`KismetSystemLibrary.Delay` 1.0)
      (goto _label_2))))

(fn `GetLockedEnemy`
  (returns (lockedEnemy :type "Actor Object Reference"))
  (return null))

(fn `OnAlert_AI?`
  (returns (Alert :type Boolean))
  (return false))

(fn `UserConstructionScript`)